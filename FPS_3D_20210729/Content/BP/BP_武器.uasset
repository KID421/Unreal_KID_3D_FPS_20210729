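; BP_武器 is a weapon Blueprint that handles automatic firing and ammo.
; While 開槍 is held and the magazine has rounds, a Delay loop spawns BP_子彈 at the muzzle socket, plays a muzzle flash and decrements ammo at the firing interval.
; Custom event 換彈匣 refills the magazine from the reserve, limited to what remains.
; Custom event 補充子彈 adds one magazine's worth to the reserve, clamped to its maximum.
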(event `InputAction|開槍`
  (params (Key :type "Key Structure"))
  (bind `_武器模型` (`self.武器模型`))
  (bind (_returnvalue_roll _returnvalue_pitch _returnvalue_yaw) (`KismetMathLibrary.BreakRotator` (`SceneComponent.GetSocketRotation` `_武器模型` "None")))
  ;[1 1 1] 開槍
  (:`Pressed`
    (set `self.開槍中` true)
    (if (and (> (`self.目前子彈數量`) 0) (`self.開槍中`)) :!label _label
      (`|SpawnActorFromClass` "/Game/BP/BP_子彈.BP_子彈_C" (`SceneComponent.GetSocketTransform` (`self.武器模型`) "子彈插槽" "RTS_World") "Undefined" "OverrideRootScale" null null) ; 生成子彈藍圖
      (`GameplayStatics.SpawnEmitterAtLocation` "/Game/InfinityBladeEffects/Effects/FX_Monsters/FX_Monster_Gruntling/Master/P_BackPack_MuzzleFlash.P_BackPack_MuzzleFlash" (`SceneComponent.GetSocketLocation` `_武器模型` "子彈插槽") (`KismetMathLibrary.MakeRotator` (+ _returnvalue_roll 90.0) _returnvalue_pitch (+ _returnvalue_yaw 90.0)) (0.08 0.08 0.08)) ; 生成粒子在指定座標上
      (set `self.目前子彈數量` (- (`self.目前子彈數量`) 1)) ; 開槍後子彈減一
      (`KismetSystemLibrary.Delay` (`self.開槍間隔`))
      (goto _label)))
  (:`Released`
    (set `self.開槍中` false)))

(event `換彈匣`
  ;[0.09532 0.4036 0.1909] 計算要補充幾顆子彈
  (set `self.要補充的子彈數量` (- (`self.彈匣尺寸`) (`self.目前子彈數量`))) ; 計算要補充的子彈數量，\n例：目前 10 彈匣 30 所以要補充 20
  ;[0.09532 0.4036 0.1909] 判斷總數是否 >= 要補充的數量
  (if (not (>= (`self.子彈總數`) (`self.要補充的子彈數量`)))
    ;[0.09532 0.4036 0.1909] 總數 < 要補充的數量：把剩餘總數補充
    (set `self.要補充的子彈數量` (`self.子彈總數`)))
  ;[0.09532 0.4036 0.1909] 目前子彈以及總數更新
  (set `self.目前子彈數量` (+ (`self.目前子彈數量`) (`self.要補充的子彈數量`))) ; 補充子彈數量，\n例：目前 10 要補充為 20 補充後 目前為 30
  (set `self.子彈總數` (- (`self.子彈總數`) (`self.要補充的子彈數量`))) ; 扣除子彈總數，\n例：總數 20 要補充為 20 補充後 總數為 0
)

(event `補充子彈`
  ;[0.09532 0.4036 0.1909] 補充子彈
  (bind _output_get (set `self.子彈總數` (+ (`self.子彈總數`) (`self.彈匣尺寸`)))) ; 子彈總數 + 彈匣尺寸
  (set `self.子彈總數` (`KismetMathLibrary.Clamp` _output_get 0 (`self.子彈上限`))))

(fn `UserConstructionScript`)