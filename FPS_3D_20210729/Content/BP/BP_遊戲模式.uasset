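; BP_遊戲模式 (game mode) runs the match countdown timer and records how many monsters need to be killed.
; BeginPlay stores the number of actors tagged "怪物" (monster) as the kill target, which is not checked here.
; Tick feeds a one-second Delay that throttles the countdown, decrementing seconds and rolling over into minutes.
; When time runs out, it zeroes the seconds and pauses the game.
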(event `self.ReceiveBeginPlay`
  ;[0.09532 0.4036 0.1909] 取得貼有怪物標籤的所有物件並儲存數量
  (bind _outactors (`GameplayStatics.GetAllActorsWithTag` "怪物"))
  (set `self.需要擊殺的怪物數量` (`KismetArrayLibrary.Array_Length` _outactors)))

(event `self.ReceiveTick`
  (params (DeltaSeconds :type "Float (single-precision)"))
  ;[1 0.3797 0.3697] 倒數系統
  ;;[1 1 1] 每秒秒數減一
  (`KismetSystemLibrary.Delay` 1.0) ; 延遲：等待所設定的時間再執行後面的節點
  (bind _output_get (set `self.秒` (- (`self.秒`) 1)))
  ;;[1 1 1] 當秒數低於 0 就把秒數設定為 59 秒
  (if (< _output_get 0)
    (set `self.秒` 59)
    ;;[1 1 1] 分大於 0 時 分減 1
    (if (> (`self.分`) 0)
      (set `self.分` (- (`self.分`) 1))
      (else
        ;;[1 1 1] 分為 0 時 秒等於 59 就代表已經沒有時間 將秒設為 0 並暫停遊戲
        (if (== (`self.秒`) 59)
          (set `self.秒` 0)
          (`GameplayStatics.SetGamePaused` true))))))

(fn `UserConstructionScript`)